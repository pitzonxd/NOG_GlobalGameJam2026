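; A key-locked door puzzle piece for the stealth game that a player opens and closes by interacting with it.
; While locked, it only responds to a StealthCharacter whose held keys include the required key ID, then unlocks permanently without removing the key.
; Once unlocked, each interaction from any actor flips the cube between hidden without collision and visible with collision, with no animation.
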(event EventOnInteract
  (params (Triggering%20Actor :type Actor%20Object%20Reference%20%28by%20ref%29))
  (bind _cube (Variables|Default|GetCube))
  (if (Variables|Default|GetIsLocked?)
    (bind _asastealth_character (Utilities|Casting|CastToAStealthCharacter Triggering%20Actor))
    (if (Utilities|Array|ContainsItem (Variables|/Game/ThiefStealthGame/Mechanics/Character/AStealthCharacter.AStealthCharacter_C|GetKeysHeld _asastealth_character) (Variables|Default|GetRequiredKeyID))
      (Variables|Default|SetIsLocked? false)
      (Utilities|FlowControl|FlipFlop :!label _label
        (:A
          (Rendering|SetVisibility _cube false true)
          (Collision|SetCollisionEnabled _cube "NoCollision"))
        (:B
          (Rendering|SetVisibility _cube true true)
          (Collision|SetCollisionEnabled _cube "QueryAndPhysics"))))
    (else
      (goto _label))))

(fn ConstructionScript)