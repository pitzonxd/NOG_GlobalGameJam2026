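; A Paper2D puzzle door that opens and closes by changing its sprite color and collision, yellow and passable or red and solid.
; Interaction toggles it according to its lock mode: unlocked, key (actor tag matching KeyID) or switch (actor tagged "Switch").
; TimedToggleDoor schedules a toggle, and any toggle clears that timer.
; DoorOpenByDefault both sets the construction-time state and tracks the current state at runtime.
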(event EventToggleDoor
  (Utilities|Time|ClearandInvalidateTimerbyHandle (Variables|Default|GetDoorTimer))
  (if (Variables|DoorPaper2D|GetDoorOpenByDefault?)
    (Variables|DoorPaper2D|SetDoorOpenByDefault? (not (Variables|DoorPaper2D|GetDoorOpenByDefault?)))
    (CallFunction|CloseDoor)
    (else
      (Variables|DoorPaper2D|SetDoorOpenByDefault? (not (Variables|DoorPaper2D|GetDoorOpenByDefault?)))
      (CallFunction|OpenDoor))))

(event EventTimedToggleDoor
  (params (Time :type Float%20%28single-precision%29))
  (bind _returnvalue (Utilities|Time|SetTimerbyEvent (delegate EventToggleDoor) Time))
  (Variables|Default|SetDoorTimer _returnvalue))

(event EventOnInteract
  (params (Triggering%20Actor :type Actor%20Object%20Reference%20%28by%20ref%29))
  (switch Utilities|FlowControl|Switch|SwitchonELockSystem (Variables|Default|GetLockSystem)
    (:NotLocked
      (Class|DoorPaper2D|ToggleDoor))
    (:LockedByKey
      (if (Actor|ActorHasTag Triggering%20Actor (Variables|Default|GetKeyID))
        (Class|DoorPaper2D|ToggleDoor :!label _label)))
    (:LockedBySwitch
      (if (Actor|ActorHasTag Triggering%20Actor "Switch")
        (goto _label)))))

(fn ConstructionScript
  (if (Variables|DoorPaper2D|GetDoorOpenByDefault?)
    (CallFunction|OpenDoor)
    (else
      (CallFunction|CloseDoor))))

(fn OpenDoor
  (bind _rendercomponent (Variables|Default|GetRenderComponent))
  (Sprite|SetSpriteColor _rendercomponent "(R=1.000000,G=0.879893,B=0.002789,A=1.000000)")
  (Collision|SetCollisionEnabled _rendercomponent "NoCollision"))

(fn CloseDoor
  (bind _rendercomponent (Variables|Default|GetRenderComponent))
  (Sprite|SetSpriteColor _rendercomponent "(R=1.000000,G=0.000012,B=0.001692,A=1.000000)")
  (Collision|SetCollisionEnabled _rendercomponent "QueryAndPhysics"))