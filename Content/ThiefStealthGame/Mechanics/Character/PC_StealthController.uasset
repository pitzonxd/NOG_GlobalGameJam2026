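; Player controller for the stealth game that adds the default input mapping and lets the player temporarily control a stealth clone.
; Spawning replaces any previous clone at the pawn's transform, hides all hide rooms, creates clone-owned copies of them, then possesses the clone.
; A 15-second timer calls RetakeControl, which unhides the original rooms, repossesses the main character, shows its HUD and updates its clone display.
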(event EventBeginPlay
  (Input|AddMappingContext (PlayerController|LocalPlayerSubsystems|GetEnhancedInputLocalPlayerSubsystem) "/Game/ThiefStealthGame/Mechanics/Character/Input/IMC_Default.IMC_Default" 0 "(bIgnoreAllPressedKeysUntilRelease=True,bForceImmediately=False,bNotifyUserSettings=False)"))

(fn ConstructionScript)

(fn SpawnCloneandTakeControl
  (bind _returnvalue (Game|Player|GetPlayerPawn 0))
  (bind _clone (Variables|Default|GetClone)
    (:then
      (Actor|DestroyActor _clone))
    (:else
      _))
  (Variables|Default|SetMainCharacter _returnvalue)
  (bind _returnvalue_2 (Game|SpawnActorfromClass "/Game/ThiefStealthGame/Mechanics/Character/AStealthClone.AStealthClone_C" (Transformation|GetActorTransform _returnvalue) "AdjustIfPossibleButAlwaysSpawn" "MultiplyWithRoot" self 0))
  (Variables|Default|SetClone _returnvalue_2)
  (bind _outactors (Actor|GetAllActorsOfClass "/Game/ThiefStealthGame/Mechanics/RoomHiding/BP_HideRoom.BP_HideRoom_C"))
  (Rendering|SetActorHiddenInGame _outactors true)
  (for _array_element _outactors
    (bind _returnvalue_3 (Game|SpawnActorfromClass "/Game/ThiefStealthGame/Mechanics/RoomHiding/BP_HideRoomClone.BP_HideRoomClone_C" (Math|Transform|MakeTransform "0, 0, 0") "Undefined" "MultiplyWithRoot" (Variables|Default|GetClone) 0))
    (Variables|/Game/ThiefStealthGame/Mechanics/RoomHiding/BP_HideRoomClone.BP_HideRoomClone_C|SetCopyRoom _returnvalue_3 _array_element)
    (Default|Copy _returnvalue_3))
  (Pawn|Possess _returnvalue_2)
  (bind _returnvalue_4 (Utilities|Time|SetTimerbyFunctionName 0 "RetakeControl" 15.0))
  (Variables|Default|SetControlTimer _returnvalue_4))

(fn RetakeControl
  (bind _maincharacter (Variables|Default|GetMainCharacter))
  (Utilities|Time|InvalidateTimerHandle (Variables|Default|GetControlTimer))
  (bind _outactors (Actor|GetAllActorsOfClass "/Game/ThiefStealthGame/Mechanics/RoomHiding/BP_HideRoom.BP_HideRoom_C"))
  (Rendering|SetActorHiddenInGame _outactors false)
  (Pawn|Possess _maincharacter)
  (bind _asastealth_character (Utilities|Casting|CastToAStealthCharacter _maincharacter))
  (Widget|SetVisibility (Variables|/Game/ThiefStealthGame/Mechanics/Character/AStealthCharacter.AStealthCharacter_C|GetHUD _asastealth_character) "Visible")
  (Default|SetCloneDisplay _asastealth_character))