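; BP_Guard is the guard in a thief stealth game, and this graph supplies the next destination along its assigned patrol path.
; GetNextPatrolPath advances an index through the path's PatrolPathPoints and wraps it to zero at the end, so the patrol loops.
; Each point is offset by the path actor's location to give a world position, without applying that actor's rotation or scale.
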(fn ConstructionScript)

(fn GetNextPatrolPath
  (bind _patrolpath (Variables|Default|GetPatrolPath))
  (bind _patrolpathpoints (Variables|/Game/ThiefStealthGame/Mechanics/Guard/PatrolPath.PatrolPath_C|GetPatrolPathPoints _patrolpath))
  (bind _result (Math|Integer|IncrementInt (Variables|Patrolling|GetIndex))
    (:%20%20
      (if (== _result (Utilities|Array|Length _patrolpathpoints))
        (Variables|Patrolling|SetIndex 0))
      (return (+ (Utilities|Array|Get(acopy) _patrolpathpoints (Variables|Patrolling|GetIndex)) (Transformation|GetActorLocation _patrolpath))))))