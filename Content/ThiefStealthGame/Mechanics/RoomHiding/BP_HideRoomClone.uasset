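; BP_HideRoomClone is a room cover that reveals its area while an AStealthClone is inside and hides it again on exit.
; Box overlaps play or reverse a timeline driving HideOpacity on the plane's dynamic material, skipping fades already at their target.
; Construction sets initial opacity from IsHidden and sizes the box slightly beyond the actor's scaled footprint.
; Copy matches transform and box to a referenced CopyRoom.
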(event OnComponentBeginOverlap(Box)
  (params (OverlappedComponent :type Primitive%20Component%20Object%20Reference) (OtherActor :type Actor%20Object%20Reference) (OtherComp :type Primitive%20Component%20Object%20Reference) (OtherBodyIndex :type Integer) (bFromSweep :type Boolean) (SweepResult :type Hit%20Result%20Structure%20%28by%20ref%29))
  (Utilities|Casting|CastToAStealthClone OtherActor)
  (CallFunction|Unhide))

(event OnComponentEndOverlap(Box)
  (params (OverlappedComponent :type Primitive%20Component%20Object%20Reference) (OtherActor :type Actor%20Object%20Reference) (OtherComp :type Primitive%20Component%20Object%20Reference) (OtherBodyIndex :type Integer))
  (Utilities|Casting|CastToAStealthClone OtherActor)
  (CallFunction|Hide))

(event Custom|Unhide
  (bind _hidematerial (Variables|Default|GetHideMaterial))
  (bind _returnvalue (Rendering|Material|GetScalarParameterValue _hidematerial "HideOpacity" :!class /Script/Engine.MaterialInstanceDynamic))
  (if (not (== _returnvalue 0.0))
    (bind _hide (Timeline|Hide&Unhide ReverseFromEnd)
      (:Update
        (Rendering|Material|SetScalarParameterValue _hidematerial "HideOpacity" _hide :!class /Script/Engine.MaterialInstanceDynamic)))))

(event Custom|Hide
  (bind _returnvalue (Rendering|Material|GetScalarParameterValue (Variables|Default|GetHideMaterial) "HideOpacity" :!class /Script/Engine.MaterialInstanceDynamic))
  (if (not (== _returnvalue 1.0))
    (bind _hide (Timeline|Hide&Unhide PlayFromStart)
      (:Update
        (Rendering|Material|SetScalarParameterValue (Variables|Default|GetHideMaterial) "HideOpacity" _hide :!class /Script/Engine.MaterialInstanceDynamic)))))

(fn ConstructionScript
  (bind _returnvalue (Transformation|GetActorScale3D))
  (bind _box (Variables|Default|GetBox))
  (bind (_x _y) (Math|Vector|BreakVector _returnvalue))
  (bind _returnvalue_2 (Rendering|Material|CreateDynamicMaterialInstance (Variables|Default|GetPlane) 0 "/Game/ThiefStealthGame/Mechanics/RoomHiding/HideMaterial.HideMaterial" "None" :!class /Script/Engine.PrimitiveComponent))
  (bind _output_get (Variables|Default|SetHideMaterial _returnvalue_2))
  (Rendering|Material|SetScalarParameterValue _output_get "HideOpacity" (Math|Float|SelectFloat 0.0 1.0 (Variables|Default|GetIsHidden?)) :!class /Script/Engine.MaterialInstanceDynamic)
  (Transformation|SetWorldScale3D _box (/ (Transformation|GetWorldScale _box) _returnvalue))
  (Components|Box|SetBoxExtent _box (Math|Vector|MakeVector (+ (* _x 5e+01) 1e+01) (+ (* _y 5e+01) 1e+01) 32.0) true))

(fn Copy
  (bind _copyroom (Variables|Default|GetCopyRoom))
  (bind _box (Variables|Default|GetBox))
  (bind _box_2 (Variables|/Game/ThiefStealthGame/Mechanics/RoomHiding/BP_HideRoom.BP_HideRoom_C|GetBox _copyroom))
  (bind _copyroom_2 (Variables|Default|GetCopyRoom)
    (:then
      (Transformation|SetActorTransform (Transformation|GetActorTransform _copyroom_2) false true)
      (Components|Box|SetBoxExtent _box (Variables|/Script/Engine.BoxComponent|GetBoxExtent _box_2) true)
      (Transformation|SetWorldScale3D _box (Transformation|GetWorldScale _box_2))
      (return))
    (:else
      (return))))