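; BP_HideRoom is a room-hiding actor that fades a plane's material to conceal or reveal an area.
; The construction script creates a dynamic material instance on the plane and sets its initial HideOpacity from the IsHidden flag.
; Hide and Unhide events play a timeline forward or in reverse to drive that parameter, skipping playback when it already sits at the respective end value.
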(event Custom|Unhide
  (bind _hidematerial (Variables|Default|GetHideMaterial))
  (bind _returnvalue (Rendering|Material|GetScalarParameterValue _hidematerial "HideOpacity" :!class /Script/Engine.MaterialInstanceDynamic))
  (if (not (== _returnvalue 0.0))
    (bind _hide (Timeline|Hide&Unhide ReverseFromEnd)
      (:Update
        (Rendering|Material|SetScalarParameterValue _hidematerial "HideOpacity" _hide :!class /Script/Engine.MaterialInstanceDynamic)))))

(event Custom|Hide
  (bind _returnvalue (Rendering|Material|GetScalarParameterValue (Variables|Default|GetHideMaterial) "HideOpacity" :!class /Script/Engine.MaterialInstanceDynamic))
  (if (not (== _returnvalue 1.0))
    (bind _hide (Timeline|Hide&Unhide PlayFromStart)
      (:Update
        (Rendering|Material|SetScalarParameterValue (Variables|Default|GetHideMaterial) "HideOpacity" _hide :!class /Script/Engine.MaterialInstanceDynamic)))))

(fn ConstructionScript
  (bind _returnvalue (Rendering|Material|CreateDynamicMaterialInstance (Variables|Default|GetPlane) 0 "/Game/ThiefStealthGame/Mechanics/RoomHiding/HideMaterial.HideMaterial" "None" :!class /Script/Engine.PrimitiveComponent))
  (bind _output_get (Variables|Default|SetHideMaterial _returnvalue))
  (Rendering|Material|SetScalarParameterValue _output_get "HideOpacity" (Math|Float|SelectFloat 0.0 1.0 (Variables|Default|GetIsHidden?)) :!class /Script/Engine.MaterialInstanceDynamic))